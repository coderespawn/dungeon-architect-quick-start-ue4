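; BP_Door_Base is a sliding double door that opens when something overlaps its Collider and closes when an overlap ends.
; The DoorAnimation timeline plays to open and reverses to close, moving DoorSlabR and DoorSlabL in opposite directions along local X, scaled by DoorDistance.
; The overlap events do not filter actors or count occupants, so any single exit starts closing the door.
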(event OnComponentBeginOverlap(Collider)
  (params (OverlappedComponent :type Primitive%20Component%20Object%20Reference) (OtherActor :type Actor%20Object%20Reference) (OtherComp :type Primitive%20Component%20Object%20Reference) (OtherBodyIndex :type Integer) (bFromSweep :type Boolean) (SweepResult :type Hit%20Result%20Structure%20%28by%20ref%29))
  (CallFunction|OpenDoor))

(event OnComponentEndOverlap(Collider)
  (params (OverlappedComponent :type Primitive%20Component%20Object%20Reference) (OtherActor :type Actor%20Object%20Reference) (OtherComp :type Primitive%20Component%20Object%20Reference) (OtherBodyIndex :type Integer))
  (CallFunction|CloseDoor))

(event Custom|OpenDoor
  (bind _doortime (Timeline|Door%20Animation Play)
    (:Update
      (Transformation|SetRelativeLocation (Variables|Default|GetDoorSlabR) (Math|Vector|MakeVector (* _doortime (Variables|Default|GetDoorDistance)) 0.0 0.0) false false)
      (Transformation|SetRelativeLocation (Variables|Default|GetDoorSlabL) (* (Math|Vector|MakeVector (* _doortime (Variables|Default|GetDoorDistance)) 0.0 0.0) -1.0) false false))))

(event Custom|CloseDoor
  (bind _doortime (Timeline|Door%20Animation Reverse)
    (:Update
      (Transformation|SetRelativeLocation (Variables|Default|GetDoorSlabR) (Math|Vector|MakeVector (* _doortime (Variables|Default|GetDoorDistance)) 0.0 0.0) false false)
      (Transformation|SetRelativeLocation (Variables|Default|GetDoorSlabL) (* (Math|Vector|MakeVector (* _doortime (Variables|Default|GetDoorDistance)) 0.0 0.0) -1.0) false false))))

(fn ConstructionScript)