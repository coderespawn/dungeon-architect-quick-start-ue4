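; Dungeon filter that bends a generated dungeon around a cylinder by rewriting its prop socket transforms when markers are emitted.
; Each socket's X position becomes an angle on a circle of twice the Radius in the XZ plane, while Y is kept.
; The circle is lowered so X = 0 lands at zero height, and each socket is pitched to follow the curve with scale unchanged.
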(fn OnMarkersEmitted
  (params (Dungeon :type Dungeon%20Object%20Reference) (PropSockets :type Array%20of%20Prop%20Socket%20Structures))
  (bind _radius (Variables|Default|GetRadius))
  (bind _returnvalue (* _radius 2.0))
  (bind _returnvalue_2 (Math|Float|MakeLiteralFloat _returnvalue))
  (for (_array_element _array_index) PropSockets
    (bind _structout (Utilities|Struct|SetmembersinPropSocket _array_element (Math|Transform|MakeTransform (- (Math|Vector|MakeVector (* (Math|Trig|Cos(Radians) (Math|Float|MultiplybyPi (+ (/ (.X (Math|Vector|BreakVector (.Location (Math|Transform|BreakTransform (.Transform (Utilities|Struct|BreakPropSocket _array_element)))))) (* (Math|Float|MultiplybyPi (Variables|Default|GetRadius)) 2.0)) 0.5))) _returnvalue_2) (.Y (Math|Vector|BreakVector (.Location (Math|Transform|BreakTransform (.Transform (Utilities|Struct|BreakPropSocket _array_element)))))) (* (Math|Trig|Sin(Radians) (Math|Float|MultiplybyPi (+ (/ (.X (Math|Vector|BreakVector (.Location (Math|Transform|BreakTransform (.Transform (Utilities|Struct|BreakPropSocket _array_element)))))) (* (Math|Float|MultiplybyPi (Variables|Default|GetRadius)) 2.0)) 0.5))) _returnvalue_2)) (Math|Vector|MakeVector 0.0 0.0 (* (Variables|Default|GetRadius) 2.0))) (Math|Rotator|CombineRotators (.Rotation (Math|Transform|BreakTransform (.Transform (Utilities|Struct|BreakPropSocket _array_element)))) (Math|Rotator|MakeRotator 0.0 (+ (Math|Trig|RadiansToDegrees (Math|Float|MultiplybyPi (+ (/ (.X (Math|Vector|BreakVector (.Location (Math|Transform|BreakTransform (.Transform (Utilities|Struct|BreakPropSocket _array_element)))))) (* (Math|Float|MultiplybyPi (Variables|Default|GetRadius)) 2.0)) 0.5))) -9e+01) 0.0)) (.Scale (Math|Transform|BreakTransform (.Transform (Utilities|Struct|BreakPropSocket _array_element)))))))
    (Utilities|Array|SetArrayElem PropSockets _array_index _structout))
  (return))