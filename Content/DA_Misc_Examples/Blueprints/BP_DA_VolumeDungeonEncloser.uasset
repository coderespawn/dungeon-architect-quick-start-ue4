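; Dungeon Architect build listener that repositions and scales an assigned Volume to enclose a grid dungeon after it is built.
; On post-build, it casts the config and model to grid types, then GetDungeonBounds folds every cell's world-space bounds into a min and max corner.
; The volume moves to their center, with zero rotation and scale from the half-extents divided by 100, plus extra height and Padding.
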(event EventOnPostDungeonBuild
  (params (Dungeon :type Dungeon%20Object%20Reference))
  (Utilities|IsValid (Variables|Default|GetVolume)
    (:Is%20Valid
      (bind _asgrid_dungeon_config (Utilities|Casting|CastToGridDungeonConfig (Variables|/Script/DungeonArchitectRuntime.Dungeon|GetConfig Dungeon)))
      (bind _asgrid_dungeon_model (Utilities|Casting|CastToGridDungeonModel (Variables|/Script/DungeonArchitectRuntime.Dungeon|GetDungeonModel Dungeon)))
      (bind (_center _scale) (CallFunction|GetDungeonBounds _asgrid_dungeon_config _asgrid_dungeon_model))
      (Transformation|SetActorTransform (Variables|Default|GetVolume) (Math|Transform|MakeTransform _center "0, 0, 0" _scale)))))

(fn GetMax
  (params (A :type Vector) (B :type Vector))
  (bind (_x _y _z) (Math|Vector|BreakVector A))
  (bind (_x_2 _y_2 _z_2) (Math|Vector|BreakVector B))
  (return (Math|Vector|MakeVector (Math|Float|Max(Float) _x _x_2) (Math|Float|Max(Float) _y _y_2) (Math|Float|Max(Float) _z _z_2))))

(fn GetMin
  (params (A :type Vector) (B :type Vector))
  (bind (_x _y _z) (Math|Vector|BreakVector A))
  (bind (_x_2 _y_2 _z_2) (Math|Vector|BreakVector B))
  (return (Math|Vector|MakeVector (Math|Float|Min(Float) _x _x_2) (Math|Float|Min(Float) _y _y_2) (Math|Float|Min(Float) _z _z_2))))

(fn GetDungeonBounds
  (params (GridConfig :type Grid%20Dungeon%20Config%20Object%20Reference) (GridModel :type Grid%20Dungeon%20Model%20Object%20Reference))
  (for (_array_element _array_index) (Variables|/Script/DungeonArchitectRuntime.GridDungeonModel|GetCells GridModel)
    (if (== _array_index 0)
      (LocalVariables|SetMin (.Location (Class|GridDungeonModelHelper|ToWorldCoords (.Bounds (Utilities|Struct|BreakCell _array_element)) (Variables|/Script/DungeonArchitectRuntime.GridDungeonConfig|GetGridCellSize GridConfig))))
      (LocalVariables|SetMax (+ (.Location (Class|GridDungeonModelHelper|ToWorldCoords (.Bounds (Utilities|Struct|BreakCell _array_element)) (Variables|/Script/DungeonArchitectRuntime.GridDungeonConfig|GetGridCellSize GridConfig))) (.Size (Class|GridDungeonModelHelper|ToWorldCoords (.Bounds (Utilities|Struct|BreakCell _array_element)) (Variables|/Script/DungeonArchitectRuntime.GridDungeonConfig|GetGridCellSize GridConfig)))))
      (else
        (Utilities|FlowControl|Sequence
          (:then_0
            (bind _min (CallFunction|GetMin (LocalVariables|GetMin) (.Location (Class|GridDungeonModelHelper|ToWorldCoords (.Bounds (Utilities|Struct|BreakCell _array_element)) (Variables|/Script/DungeonArchitectRuntime.GridDungeonConfig|GetGridCellSize GridConfig)))))
            (LocalVariables|SetMin _min))
          (:then_1
            (bind _max (CallFunction|GetMax (+ (.Location (Class|GridDungeonModelHelper|ToWorldCoords (.Bounds (Utilities|Struct|BreakCell _array_element)) (Variables|/Script/DungeonArchitectRuntime.GridDungeonConfig|GetGridCellSize GridConfig))) (.Size (Class|GridDungeonModelHelper|ToWorldCoords (.Bounds (Utilities|Struct|BreakCell _array_element)) (Variables|/Script/DungeonArchitectRuntime.GridDungeonConfig|GetGridCellSize GridConfig)))) (LocalVariables|GetMax)))
            (LocalVariables|SetMax _max))))))
  (return (/ (+ (LocalVariables|GetMin) (LocalVariables|GetMax)) 2.0) (+ (+ (/ (/ (- (LocalVariables|GetMax) (LocalVariables|GetMin)) 2.0) 1e+02) "0, 0,1.000000") (Variables|Default|GetPadding))))