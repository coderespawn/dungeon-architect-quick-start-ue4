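; Dungeon Architect example Blueprint that fits spawn room and boss room volumes around rooms in a grid dungeon.
; When the layout is built, it takes the two furthest rooms from the grid query and uses their cell centers and sizes.
; SetVolumeBounds moves each valid volume to its room center, converting size to actor scale with extra height and padding.
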(event EventOnDungeonLayoutBuilt
  (params (Dungeon :type Dungeon%20Object%20Reference))
  (bind _asgrid_dungeon_query (Utilities|Casting|CastToGridDungeonQuery (Class|Dungeon|GetQuery Dungeon)))
  (CallFunction|SetVolumeBounds (Variables|Default|GetSpawnRoomVolume) (.OutCenter (Class|GridDungeonQuery|GetCellDimension _asgrid_dungeon_query (.OutRoomA (Class|GridDungeonQuery|GetFurthestRooms _asgrid_dungeon_query)))) (.OutSize (Class|GridDungeonQuery|GetCellDimension _asgrid_dungeon_query (.OutRoomA (Class|GridDungeonQuery|GetFurthestRooms _asgrid_dungeon_query)))))
  (CallFunction|SetVolumeBounds (Variables|Default|GetBossRoomVolume) (.OutCenter (Class|GridDungeonQuery|GetCellDimension _asgrid_dungeon_query (.OutRoomB (Class|GridDungeonQuery|GetFurthestRooms _asgrid_dungeon_query)))) (.OutSize (Class|GridDungeonQuery|GetCellDimension _asgrid_dungeon_query (.OutRoomB (Class|GridDungeonQuery|GetFurthestRooms _asgrid_dungeon_query))))))

(fn SetVolumeBounds
  (params (Volume :type Volume%20Object%20Reference) (Center :type Vector) (Scale :type Vector))
  (Utilities|IsValid Volume
    (:Is%20Valid
      (Transformation|SetActorTransform Volume (Math|Transform|MakeTransform Center "0, 0, 0" (+ (+ (/ Scale 2e+02) "0, 0,1.000000") (Variables|Default|GetPadding))) false true))))