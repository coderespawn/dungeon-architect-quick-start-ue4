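; Elevator cabin actor that travels vertically between BP_LiftHolder floor stops.
; On BeginPlay it registers holders within a horizontal radius and passes the floor count to its child-actor BP_LiftPanel.
; Panel presses call the holder nearest the floor's height; MoveToFloor closes all doors and sets the target.
; Tick moves the cabin at constant speed, clamping the last step, updates the panel's floor display, then releases buttons and notifies the holder on arrival.
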(event EventBeginPlay
  (bind _asbp_lift_panel (Utilities|Casting|CastToBP_LiftPanel (Variables|/Script/Engine.ChildActorComponent|GetChildActor (Variables|Default|GetBP_LiftPanel))))
  (bind _output_get (Variables|Default|SetLiftPanelCast _asbp_lift_panel))
  (EventDispatchers|BindEventtoOnPanelButtonPressedEvent _output_get (EventDispatchers|CreateEvent :!event OnPanelButtonPressed))
  (CallFunction|InitializeFloors))

(event Collision|EventActorBeginOverlap
  (params (OtherActor :type Actor%20Object%20Reference)))

(event EventTick
  (params (DeltaSeconds :type Float%20%28single-precision%29))
  (CallFunction|ProcessMoveLift DeltaSeconds))

(fn ConstructionScript)

(fn InitializeFloors
  (Utilities|Array|Clear (Variables|Default|GetLiftHolders))
  (bind _outactors (Actor|GetAllActorsOfClass "/Game/DA_Floorplan_Demo/Art/Blueprints/BP_LiftHolder.BP_LiftHolder_C"))
  (for _array_element _outactors
    (if (< (Math|Vector|VectorLength (* (- (Transformation|GetActorLocation _array_element) (Transformation|GetActorLocation)) "1.000000,1.000000,0.000000")) (Variables|Default|GetLiftHolderProximityRadius))
      (Variables|/Game/DA_Floorplan_Demo/Art/Blueprints/BP_LiftHolder.BP_LiftHolder_C|SetCabin _array_element self)
      (Utilities|Array|Add (Variables|Default|GetLiftHolders) _array_element)))
  (bind _output_get (Variables|Default|SetNumFloors (Utilities|Array|Length (Variables|Default|GetLiftHolders))))
  (Default|SetNumFloors (Variables|Default|GetLiftPanelCast) _output_get))

(fn MovetoFloor
  (params (FloorDoor :type BP%20Lift%20Holder%20Object%20Reference))
  (if (not (Variables|Default|GetIsMoving))
    (Variables|Default|SetIsMoving true)
    (Variables|Default|SetTargetFloor FloorDoor)
    (CallFunction|CloseAllDoors)))

(fn ProcessMoveLift
  (params (DeltaTime :type Float%20%28single-precision%29))
  (bind _returnvalue (Transformation|GetActorLocation))
  (bind _targetfloor (Variables|Default|GetTargetFloor))
  (bind _returnvalue_2 (Transformation|GetActorLocation _targetfloor))
  (bind _returnvalue_3 (- _returnvalue_2 _returnvalue))
  (bind _returnvalue_4 (* _returnvalue_3 "0, 0,1.000000"))
  (if (Variables|Default|GetIsMoving)
    (Utilities|IsValid (Variables|Default|GetTargetFloor)
      (:Is%20Valid
        (LocalVariables|SetFrameMoveDistance (* DeltaTime (Variables|Default|GetMovementPerSecond)))
        (LocalVariables|SetDistanceToTarget (Math|Vector|VectorLength _returnvalue_4))
        (LocalVariables|SetMoveDirection (Math|Vector|Normalize _returnvalue_4))
        (if (<= (LocalVariables|GetDistanceToTarget) (LocalVariables|GetFrameMoveDistance))
          (LocalVariables|SetFrameMoveDistance (LocalVariables|GetDistanceToTarget)))
        (Transformation|SetActorLocation (+ (Transformation|GetActorLocation) (* (LocalVariables|GetMoveDirection) (LocalVariables|GetFrameMoveDistance))) false false)
        (bind _asbp_lift_panel (Utilities|Casting|CastToBP_LiftPanel (Variables|/Script/Engine.ChildActorComponent|GetChildActor (Variables|Default|GetBP_LiftPanel))))
        (Default|SetCurrentFloor _asbp_lift_panel (Math|Float|Round (/ (.Z (Math|Vector|BreakVector (+ (Transformation|GetActorLocation) (* (LocalVariables|GetMoveDirection) (LocalVariables|GetFrameMoveDistance))))) (Variables|Default|GetFloorHeight))))
        (if (<= (LocalVariables|GetDistanceToTarget) (LocalVariables|GetFrameMoveDistance))
          (CallFunction|NotifyReachedDestination))))))

(fn NotifyReachedDestination
  (Utilities|IsValid (Variables|Default|GetTargetFloor)
    (:Is%20Valid
      (Default|ReleaseAllPanelButtons (Variables|Default|GetLiftPanelCast))
      (Default|OnLiftReachedFloor (Variables|Default|GetTargetFloor))
      (Variables|Default|SetIsMoving false)
      (Variables|Default|SetTargetFloor 0))))

(fn GetFloorHolderat
  (params (Index :type Integer))
  (LocalVariables|SetTargetHeight (* Index (Variables|Default|GetFloorHeight)))
  (for _array_element (Variables|Default|GetLiftHolders)
    (if (< (Math|Float|Absolute(Float) (- (.Z (Math|Vector|BreakVector (Transformation|GetActorLocation _array_element))) (LocalVariables|GetTargetHeight))) (LocalVariables|GetBestDistance))
      (LocalVariables|SetBestDistance (Math|Float|Absolute(Float) (- (.Z (Math|Vector|BreakVector (Transformation|GetActorLocation _array_element))) (LocalVariables|GetTargetHeight))))
      (LocalVariables|SetBestFloor _array_element)))
  (return (LocalVariables|GetBestFloor)))

(fn OnPanelButtonPressed
  (params (FloorIndex :type Integer) (Button :type BP%20Pushable%20Button%20Object%20Reference))
  (if (not (Variables|Default|GetIsMoving))
    (Default|PushButton Button)
    (bind _floor (CallFunction|GetFloorHolderat FloorIndex))
    (Default|CallLift _floor)))

(fn CloseAllDoors
  (for _array_element (Variables|Default|GetLiftHolders)
    (Default|CloseDoor _array_element)))