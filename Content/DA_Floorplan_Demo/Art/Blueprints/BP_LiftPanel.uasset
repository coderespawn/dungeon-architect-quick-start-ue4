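; Lift control panel with floor buttons and a text display for the current floor.
; The construction script gathers eight child-actor BP_PushableButtons, labels and binds one per floor up to NumFloors (index 0 shows "G"), and disables the rest.
; Each button carries its floor index as UserData, which the panel rebroadcasts through an event on press.
; SetCurrentFloor updates the display and highlights the matching button, and ReleaseAllPanelButtons releases every button.
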(event EventBeginPlay)

(event Collision|EventActorBeginOverlap
  (params (OtherActor :type Actor%20Object%20Reference)))

(event EventTick
  (params (DeltaSeconds :type Float%20%28single-precision%29)))

(fn ConstructionScript
  (CallFunction|SetNumFloors (Variables|Default|GetNumFloors)))

(fn SetNumFloors
  (params (Count :type Integer))
  (Variables|Default|SetNumFloors Count)
  (Utilities|FlowControl|Sequence
    (:then_0
      ;[1 1 1] Grab references to the buttons in the panel
      (Utilities|Array|Clear (Variables|Default|GetButtons))
      (for _array_element (Utilities|Array|MakeArray (Variables|Default|GetButtonFloor7) (Variables|Default|GetButtonFloor8) (Variables|Default|GetButtonFloor5) (Variables|Default|GetButtonFloor6) (Variables|Default|GetButtonFloor3) (Variables|Default|GetButtonFloor4) (Variables|Default|GetButtonFloor1) (Variables|Default|GetButtonFloor2))
        (bind _asbp_pushable_button (Utilities|Casting|CastToBP_PushableButton (Variables|/Script/Engine.ChildActorComponent|GetChildActor _array_element)))
        (Utilities|Array|Add (Variables|Default|GetButtons) _asbp_pushable_button)))
    (:then_1
      (for (_array_element_2 _array_index) (Variables|Default|GetButtons)
        (if (< (+ _array_index 0) (Variables|Default|GetNumFloors))
          (bind _text (CallFunction|GetFloorText (+ _array_index 0)))
          (Default|SetButtonText _array_element_2 _text)
          (Variables|/Game/DA_Floorplan_Demo/Art/Blueprints/BP_PushableButton.BP_PushableButton_C|SetUserData _array_element_2 (+ _array_index 0))
          (EventDispatchers|BindEventtoOnButtonPressedDelegate _array_element_2 (EventDispatchers|CreateEvent :!event OnPanelButtonPressed))
          (else
            (Utilities|IsValid _array_element_2
              (:Is%20Valid
                (Default|DisableButton _array_element_2)))))))))

(fn OnPanelButtonPressed
  (params (Button :type BP%20Pushable%20Button%20Object%20Reference))
  (Default|CallOnPanelButtonPressedEvent (Variables|/Game/DA_Floorplan_Demo/Art/Blueprints/BP_PushableButton.BP_PushableButton_C|GetUserData Button) Button))

(fn GetFloorText
  (params (Index :type Integer))
  (if (== Index 0)
    (return "G")
    (else
      (return (Utilities|Text|ToText(Integer) Index)))))

(fn SetCurrentFloor
  (params (FloorIndex :type Integer))
  (if (!= FloorIndex (Variables|Default|GetPanelDisplayFloorIndex))
    (bind _output_get (Variables|Default|SetPanelDisplayFloorIndex FloorIndex))
    (bind _text (CallFunction|GetFloorText _output_get))
    (Rendering|Components|TextRender|SetText (Variables|Default|GetNewTextRenderComponent) _text)
    (for _array_element (Variables|Default|GetButtons)
      (Variables|/Game/DA_Floorplan_Demo/Art/Blueprints/BP_PushableButton.BP_PushableButton_C|SetIsHilighted _array_element (== (Variables|/Game/DA_Floorplan_Demo/Art/Blueprints/BP_PushableButton.BP_PushableButton_C|GetUserData _array_element) _output_get))
      (Default|UpdateButtonState _array_element (Variables|/Game/DA_Floorplan_Demo/Art/Blueprints/BP_PushableButton.BP_PushableButton_C|GetButtonState _array_element)))))

(fn ReleaseAllPanelButtons
  (for _array_element (Variables|Default|GetButtons)
    (Default|ReleaseButton _array_element)))