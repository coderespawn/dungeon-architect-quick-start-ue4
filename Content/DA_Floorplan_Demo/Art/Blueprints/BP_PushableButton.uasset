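; BP_PushableButton is an interactive button with a text label and a ring mesh whose material shows its state.
; UpdateButtonState swaps the ring material for Normal, Hover, Pushed or Disabled, with a highlight variant of Normal.
; Hover and press events pass through an IsEnabled macro; hover leaves pushed buttons unchanged.
; Pressing only broadcasts a delegate with itself, while separate functions push, release or disable the button.
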(event Custom|OnHoverIn
  (Utilities|IsEnabled
    (:Enabled
      (if (Utilities|Enum|NotEqual(Enum) (Variables|Default|GetButtonState) "NewEnumerator2")
        (CallFunction|UpdateButtonState "NewEnumerator1")))))

(event Custom|OnHoverOut
  (Utilities|IsEnabled
    (:Enabled
      (if (Utilities|Enum|NotEqual(Enum) (Variables|Default|GetButtonState) "NewEnumerator2")
        (CallFunction|UpdateButtonState "NewEnumerator0")))))

(event Custom|OnButtonPressed
  (Utilities|IsEnabled
    (:Enabled
      (Default|CallOnButtonPressedDelegate self))))

(event EventBeginPlay)

(event Collision|EventActorBeginOverlap
  (params (OtherActor :type Actor%20Object%20Reference)))

(event EventTick
  (params (DeltaSeconds :type Float%20%28single-precision%29)))

(fn ConstructionScript)

(fn SetButtonText
  (params (Text :type Text))
  (Rendering|Components|TextRender|SetText (Variables|Default|GetText) Text))

(fn DisableButton
  (CallFunction|UpdateButtonState "NewEnumerator4"))

(fn UpdateButtonState
  (params (State :type E_PushableButtonStates%20Enum))
  (bind _buttonring (Variables|Default|GetButtonRing))
  (bind _output_get (Variables|Default|SetButtonState State))
  (switch Utilities|FlowControl|Switch|SwitchonE_PushableButtonStates _output_get
    (:NewEnumerator0
      (if (Variables|Default|GetIsHilighted)
        (Rendering|Material|SetMaterial _buttonring 0 (Variables|Default|GetHilightMaterial))
        (else
          (Rendering|Material|SetMaterial _buttonring 0 (Variables|Default|GetNormalMaterial)))))
    (:NewEnumerator1
      (Rendering|Material|SetMaterial (Variables|Default|GetButtonRing) 0 (Variables|Default|GetHoverMaterial)))
    (:NewEnumerator2
      (Rendering|Material|SetMaterial (Variables|Default|GetButtonRing) 0 (Variables|Default|GetPushedMaterial)))
    (:NewEnumerator4
      (Rendering|Material|SetMaterial (Variables|Default|GetButtonRing) 0 (Variables|Default|GetDisabledMaterial)))))

(fn PushButton
  (CallFunction|UpdateButtonState "NewEnumerator2"))

(fn ReleaseButton
  (if (Utilities|Enum|Equal(Enum) (Variables|Default|GetButtonState) "NewEnumerator2")
    (CallFunction|UpdateButtonState "NewEnumerator0")))