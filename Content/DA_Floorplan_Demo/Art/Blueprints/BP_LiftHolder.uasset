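; BP_LiftHolder is a lift landing with a call button and two sliding doors, serving as a floor that the cabin can be sent to.
; Pressing the child-actor button runs CallLift, which latches the button and sends the referenced Cabin to this actor.
; OnLiftReachedFloor releases the button and opens the doors along a timeline, offset from their cached start positions.
; Tick counts the open time and reverses the timeline to auto-close them.
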(event Custom|OpenDoor
  (Variables|Default|SetIsDoorOpen true)
  (Variables|Default|SetTimeSinceDoorOpened 0.0)
  (bind _openanim (Timeline|DoorAnimation Play)
    (:Update
      (Transformation|SetRelativeLocation (Variables|Default|GetDoor1) (- (Variables|Default|GetDoor1BaseLoc) (Math|Vector|MakeVector 0.0 (* _openanim (Variables|Default|GetDoorOpenDistance)) 0.0)) false false)
      (Transformation|SetRelativeLocation (Variables|Default|GetDoor2) (+ (Math|Vector|MakeVector 0.0 (* _openanim (Variables|Default|GetDoorOpenDistance)) 0.0) (Variables|Default|GetDoor2BaseLoc)) false false))))

(event Custom|OnCallButtonPressed
  (params (Button :type BP%20Pushable%20Button%20Object%20Reference))
  (CallFunction|CallLift))

(event Custom|OnLiftReachedFloor
  (Default|ReleaseButton (Variables|Default|GetCallButtonCast))
  (CallFunction|OpenDoor))

(event Custom|CloseDoor
  (Variables|Default|SetIsDoorOpen false)
  (bind _openanim (Timeline|DoorAnimation Reverse)
    (:Update
      (Transformation|SetRelativeLocation (Variables|Default|GetDoor1) (- (Variables|Default|GetDoor1BaseLoc) (Math|Vector|MakeVector 0.0 (* _openanim (Variables|Default|GetDoorOpenDistance)) 0.0)) false false)
      (Transformation|SetRelativeLocation (Variables|Default|GetDoor2) (+ (Math|Vector|MakeVector 0.0 (* _openanim (Variables|Default|GetDoorOpenDistance)) 0.0) (Variables|Default|GetDoor2BaseLoc)) false false))))

(event EventBeginPlay
  (bind _asbp_pushable_button (Utilities|Casting|CastToBP_PushableButton (Variables|/Script/Engine.ChildActorComponent|GetChildActor (Variables|Default|GetCallButton))))
  (Variables|Default|SetCallButtonCast _asbp_pushable_button)
  (Variables|Default|SetDoor1BaseLoc (Variables|/Script/Engine.SceneComponent|GetRelativeLocation (Variables|Default|GetDoor1)))
  (Variables|Default|SetDoor2BaseLoc (Variables|/Script/Engine.SceneComponent|GetRelativeLocation (Variables|Default|GetDoor2)))
  (bind _asbp_pushable_button_2 (Utilities|Casting|CastToBP_PushableButton (Variables|/Script/Engine.ChildActorComponent|GetChildActor (Variables|Default|GetCallButton))))
  (EventDispatchers|BindEventtoOnButtonPressedDelegate _asbp_pushable_button_2 (delegate Custom|OnCallButtonPressed)))

(event Collision|EventActorBeginOverlap
  (params (OtherActor :type Actor%20Object%20Reference)))

(event EventTick
  (params (DeltaSeconds :type Float%20%28single-precision%29))
  (Utilities|FlowControl|Sequence
    (:then_0
      (if (Variables|Default|GetIsDoorOpen)
        (bind _output_get (Variables|Default|SetTimeSinceDoorOpened (+ DeltaSeconds (Variables|Default|GetTimeSinceDoorOpened))))
        (if (> _output_get (Variables|Default|GetTimeTillAutoClose))
          (CallFunction|CloseDoor))))))

(fn ConstructionScript)

(fn CallLift
  (Utilities|IsValid (Variables|Default|GetCabin)
    (:Is%20Valid
      (Default|PushButton (Variables|Default|GetCallButtonCast))
      (Default|MovetoFloor (Variables|Default|GetCabin) self))))