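; Dungeon Architect marker post-processor in the Isaac demo that removes markers sharing the same position.
; OnMarkersEmitted walks the emitted marker list, keeping the first marker at each transform location and recording that location in VisitedLocation.
; It returns the filtered TargetMarkerList, comparing only exact locations and ignoring any other marker properties.
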(fn OnMarkersEmitted
  (params (Dungeon :type Dungeon%20Object%20Reference) (MarkerList :type Array%20of%20Dungeon%20Marker%20Info%20Structures))
  (for _array_element MarkerList
    (if (not (Utilities|Set|Contains (LocalVariables|GetVisitedLocation) (.Location (Math|Transform|BreakTransform (.transform (Utilities|Struct|BreakDungeonMarkerInfo _array_element))))))
      (Utilities|Array|Add (LocalVariables|GetTargetMarkerList) _array_element)
      (Utilities|Set|Add (LocalVariables|GetVisitedLocation) (.Location (Math|Transform|BreakTransform (.transform (Utilities|Struct|BreakDungeonMarkerInfo _array_element)))))))
  (return (LocalVariables|GetTargetMarkerList)))