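; Isaac-style dungeon camera actor that takes over the first player's view and glides to the center of the room containing the player.
; BeginPlay reads room size and padding from the Dungeon's IsaacDungeonConfig.
; Each Tick, UpdateCamPosition floors the player's location onto the padded room grid to find that center.
; The actor then teleports a fixed fraction toward it with zero rotation, giving a frame-rate-dependent smooth pan.
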(event EventBeginPlay
  (bind _asisaac_dungeon_config (Utilities|Casting|CastToIsaacDungeonConfig (Variables|/Script/DungeonArchitectRuntime.Dungeon|GetConfig (Variables|Default|GetDungeon))))
  (Variables|Default|SetRoomPadding (Variables|/Script/DungeonArchitectRuntime.IsaacDungeonConfig|GetRoomPadding _asisaac_dungeon_config))
  (Variables|Default|SetRoomSize (* (Math|Vector|MakeVector (Math|Conversions|ToFloat(Integer) (Variables|/Script/DungeonArchitectRuntime.IsaacDungeonConfig|GetRoomWidth _asisaac_dungeon_config)) (Math|Conversions|ToFloat(Integer) (Variables|/Script/DungeonArchitectRuntime.IsaacDungeonConfig|GetRoomLength _asisaac_dungeon_config)) 0.0) (Variables|/Script/DungeonArchitectRuntime.IsaacDungeonConfig|GetTileSize _asisaac_dungeon_config)))
  (Game|Player|SetViewTargetwithBlend (Game|GetPlayerController 0) self 0.0 "VTBlend_EaseOut" 0.5 false))

(event EventActorBeginOverlap
  (params (OtherActor :type Actor%20Object%20Reference)))

(event EventTick
  (params (DeltaSeconds :type Float%20%28single-precision%29))
  (CallFunction|UpdateCamPosition)
  (Transformation|Teleport (Math|Interpolation|Ease "Linear" 0.1 (Transformation|GetActorLocation self) (Variables|Default|GetTargetPosition)) "0, 0, 0"))

(fn ConstructionScript)

(fn UpdateCamPosition
  (bind _location (CallFunction|GetPlayerLocation))
  (bind _roomsize (Variables|Default|GetRoomSize))
  (bind _roompadding (Variables|Default|GetRoomPadding))
  (bind _returnvalue (+ _roomsize _roompadding))
  (bind _returnvalue_2 (+ _returnvalue "0, 0,1.000000"))
  (bind _returnvalue_3 (/ _location _returnvalue_2))
  (bind (_x _y) (Math|Vector|BreakVector _returnvalue_3))
  (Variables|Default|SetTargetPosition (+ (* (Math|Vector|MakeVector (Math|Conversions|ToFloat(Integer) (Math|Float|Floor _x)) (Math|Conversions|ToFloat(Integer) (Math|Float|Floor _y)) 0.0) (+ (Variables|Default|GetRoomSize) (Variables|Default|GetRoomPadding))) (/ (Variables|Default|GetRoomSize) 2.0))))

(fn GetPlayerLocation
  (return (Transformation|GetActorLocation (Game|Player|GetPlayerPawn 0))))