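; Dungeon marker emitter that places a single "LowestPoint" marker beneath a grid dungeon's overall footprint.
; It converts each looped element's grid bounds to world space and merges them into one bounding box using the component-wise GetMin and GetMax helpers.
; The marker sits at the box's XY center and minimum Z, with XY scaled to extent/100 so a 100-unit mesh spans the whole layout.
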(event EventEmitMarkers
  (params (Builder :type Dungeon%20Builder%20Object%20Reference) (Model :type Dungeon%20Model%20Object%20Reference) (Config :type Dungeon%20Config%20Object%20Reference) (Query :type Dungeon%20Query%20Object%20Reference))
  (bind _asgrid_dungeon_config (Utilities|Casting|CastToGridDungeonConfig Config))
  (for (_array_element _array_index) 0
    (if (== _array_index 0)
      (Variables|Default|SetMin (.Location (Class|GridDungeonModelHelper|ToWorldCoords (.Bounds (Utilities|Struct|BreakCell _array_element)) (Variables|/Script/DungeonArchitectRuntime.GridDungeonConfig|GetGridCellSize _asgrid_dungeon_config))))
      (Variables|Default|SetMax (+ (.Location (Class|GridDungeonModelHelper|ToWorldCoords (.Bounds (Utilities|Struct|BreakCell _array_element)) (Variables|/Script/DungeonArchitectRuntime.GridDungeonConfig|GetGridCellSize _asgrid_dungeon_config))) (.Size (Class|GridDungeonModelHelper|ToWorldCoords (.Bounds (Utilities|Struct|BreakCell _array_element)) (Variables|/Script/DungeonArchitectRuntime.GridDungeonConfig|GetGridCellSize _asgrid_dungeon_config)))))
      (else
        (Utilities|FlowControl|Sequence
          (:then_0
            (bind _min (CallFunction|GetMin (Variables|Default|GetMin) (.Location (Class|GridDungeonModelHelper|ToWorldCoords (.Bounds (Utilities|Struct|BreakCell _array_element)) (Variables|/Script/DungeonArchitectRuntime.GridDungeonConfig|GetGridCellSize _asgrid_dungeon_config)))))
            (Variables|Default|SetMin _min))
          (:then_1
            (bind _max (CallFunction|GetMax (+ (.Location (Class|GridDungeonModelHelper|ToWorldCoords (.Bounds (Utilities|Struct|BreakCell _array_element)) (Variables|/Script/DungeonArchitectRuntime.GridDungeonConfig|GetGridCellSize _asgrid_dungeon_config))) (.Size (Class|GridDungeonModelHelper|ToWorldCoords (.Bounds (Utilities|Struct|BreakCell _array_element)) (Variables|/Script/DungeonArchitectRuntime.GridDungeonConfig|GetGridCellSize _asgrid_dungeon_config)))) (Variables|Default|GetMax)))
            (Variables|Default|SetMax _max))))))
  (bind _output_get (Variables|Default|SetCenter (/ (+ (Variables|Default|GetMin) (Variables|Default|GetMax)) 2.0)))
  (Class|DungeonBuilder|EmitMarker Builder "LowestPoint" (Math|Transform|MakeTransform (Math|Vector|MakeVector (.X (Math|Vector|BreakVector _output_get)) (.Y (Math|Vector|BreakVector _output_get)) (.Z (Math|Vector|BreakVector (Variables|Default|GetMin)))) "0, 0, 0" (Math|Vector|MakeVector (.X (Math|Vector|BreakVector (/ (/ (- (Variables|Default|GetMax) (Variables|Default|GetMin)) 2.0) 5e+01))) (.Y (Math|Vector|BreakVector (/ (/ (- (Variables|Default|GetMax) (Variables|Default|GetMin)) 2.0) 5e+01))) 1.0))))

(fn GetMin
  (params (A :type Vector) (B :type Vector))
  (bind (_x _y _z) (Math|Vector|BreakVector A))
  (bind (_x_2 _y_2 _z_2) (Math|Vector|BreakVector B))
  (return (Math|Vector|MakeVector (Math|Float|Min(Float) _x _x_2) (Math|Float|Min(Float) _y _y_2) (Math|Float|Min(Float) _z _z_2))))

(fn GetMax
  (params (A :type Vector) (B :type Vector))
  (bind (_x _y _z) (Math|Vector|BreakVector A))
  (bind (_x_2 _y_2 _z_2) (Math|Vector|BreakVector B))
  (return (Math|Vector|MakeVector (Math|Float|Max(Float) _x _x_2) (Math|Float|Max(Float) _y _y_2) (Math|Float|Max(Float) _z _z_2))))