(event Custom|OnStateBuild
  (bind _returnvalue (Math|Transform|MakeTransform "0, 0,0.000000" "0,0.000000, 0"))
  (bind _returnvalue_2 (Game|SpawnActorfromClass "/Game/DA_StarterPack/LevelBuilderGame/Blueprints/BP_DALB_BuildGrid.BP_DALB_BuildGrid_C" _returnvalue "AlwaysSpawn" 0 0))
  (bind _output_get (Variables|Default|SetBuildGrid _returnvalue_2))
  (Default|SetGridSize _output_get (Variables|Default|GetGridCellSize))
  (bind _returnvalue_3 (Game|SpawnActorfromClass "/Game/DA_StarterPack/LevelBuilderGame/Blueprints/BP_DALB_BuildGridCursor.BP_DALB_BuildGridCursor_C" _returnvalue "AlwaysSpawn" 0 0))
  (bind _output_get_2 (Variables|Default|SetBuildGridCursor _returnvalue_3))
  (Default|SetGridSize _output_get_2 (Variables|Default|GetGridCellSize)))

(event Custom|OnStateSimulate
  (Actor|DestroyActor (Variables|Default|GetBuildGrid))
  (Actor|DestroyActor (Variables|Default|GetBuildGridCursor)))

(event EventBeginPlay
  (bind _asbp_dalb_game_state (Utilities|Casting|CastToBP_DALB_GameState (Game|GetGameState)))
  (bind _output_get (Variables|Default|SetGameState _asbp_dalb_game_state))
  (EventDispatchers|BindEventtoOnStateChangeBuild _output_get (delegate Custom|OnStateBuild))
  (EventDispatchers|BindEventtoOnStateChangeSimulate _output_get (delegate Custom|OnStateSimulate)))

(event EventTick
  (params (DeltaSeconds :type Float%20%28single-precision%29))
  (Utilities|FlowControl|Sequence
    (:then_0
      (CallFunction|HandleFrameInput DeltaSeconds))
    (:then_1
      (bind _asbp_dalb_game_state (Utilities|Casting|CastToBP_DALB_GameState (Game|GetGameState)))
      (switch Utilities|FlowControl|Switch|SwitchonDALB_GameStateTypes (Variables|/Game/DA_StarterPack/LevelBuilderGame/Blueprints/Game/BP_DALB_GameState.BP_DALB_GameState_C|GetCurrentStateType _asbp_dalb_game_state)
        (:NewEnumerator0
          (CallFunction|HandleGameSimulate DeltaSeconds))
        (:NewEnumerator1
          (CallFunction|HandleGameBuild DeltaSeconds))))))

(event Input|KeyboardEvents|SpaceBar
  (params (Key :type Key%20Structure))
  (:Pressed
    (bind _asbp_dalb_game_state (Utilities|Casting|CastToBP_DALB_GameState (Game|GetGameState)))
    (Utilities|FlowControl|FlipFlop
      (:A
        (Default|ChangetoState _asbp_dalb_game_state "NewEnumerator0"))
      (:B
        (Default|ChangetoState _asbp_dalb_game_state "NewEnumerator1")))))

(event Input|MouseEvents|LeftMouseButton
  (params (Key :type Key%20Structure))
  (:Pressed
    (Variables|Default|SetIsBuildingCell true))
  (:Released
    (Variables|Default|SetIsBuildingCell false)))

(event Input|MouseEvents|RightMouseButton
  (params (Key :type Key%20Structure))
  (:Pressed
    (Variables|Default|SetIsDestroyingCell true))
  (:Released
    (Variables|Default|SetIsDestroyingCell false)))

(event Input|MouseEvents|MouseWheelUp
  (params (Key :type Key%20Structure))
  (:Pressed
    (Variables|Default|SetBuildFloorIndex (+ (Variables|Default|GetBuildFloorIndex) 1))))

(event Input|MouseEvents|MouseWheelDown
  (params (Key :type Key%20Structure))
  (:Pressed
    (Variables|Default|SetBuildFloorIndex (- (Variables|Default|GetBuildFloorIndex) 1))))

(fn ConstructionScript)

(fn HandleFrameInput
  (params (DeltaSeconds :type Float%20%28single-precision%29))
  (Pawn|Input|AddMovementInput (Math|Vector|MakeVector (Input|AxisValues|GetMoveForward) (Input|AxisValues|GetMoveRight) 0.0) 1.0 false))

(fn HandleGameSimulate
  (params (DeltaSeconds :type Float%20%28single-precision%29)))

(fn HandleGameBuild
  (params (DeltaSeconds :type Float%20%28single-precision%29))
  (bind _returnvalue (Game|GetPlayerController 0))
  (bind _buildfloorindex (Variables|Default|GetBuildFloorIndex))
  (bind _gridcellsize (Variables|Default|GetGridCellSize))
  (bind (_worldlocation _worlddirection) (Game|Player|ConvertMouseLocationToWorldSpace _returnvalue))
  (bind _z (Math|Vector|BreakVector _gridcellsize))
  (bind _returnvalue_2 (* _worlddirection 5e+03))
  (bind _returnvalue_3 (* _buildfloorindex _z))
  (bind _returnvalue_4 (Math|Vector|MakeVector 0.0 0.0 _returnvalue_3))
  (bind _returnvalue_5 (+ _worldlocation _returnvalue_2))
  (bind (_t _intersection _returnvalue_6) (Class|KismetMathLibrary|LinePlaneIntersectionOriginNormal _worldlocation _returnvalue_5 _returnvalue_4 "0, 0,1.000000"))
  (Utilities|FlowControl|Sequence
    (:then_0
      ;[1 1 1] Calculate the cursor position
      (if _returnvalue_6
        (bind _result (CallFunction|DivideFloor _intersection (Variables|Default|GetGridCellSize)))
        (Variables|Default|SetGridCursorPosition (Math|Vector|MakeVector (.X (Math|Vector|BreakVector _result)) (.Y (Math|Vector|BreakVector _result)) (Math|Conversions|ToFloat(Integer) (Variables|Default|GetBuildFloorIndex))))
        (CallFunction|UpdateGridCursorPosition)
        (Variables|/Script/DungeonArchitectRuntime.Dungeon|SetBuildPriorityLocation (Variables|/Game/DA_StarterPack/LevelBuilderGame/Blueprints/Game/BP_DALB_GameState.BP_DALB_GameState_C|GetDungeon (Variables|Default|GetGameState)) (* (Variables|Default|GetGridCellSize) (Variables|Default|GetGridCursorPosition)))))
    (:then_1
      ;[1 1 1] Handle Build Cell
      (if (Variables|Default|GetIsBuildingCell)
        (Default|AddPaintedCell (Variables|Default|GetGameState) (Variables|Default|GetGridCursorPosition))))
    (:then_2
      ;[1 1 1] Handle Destroy Cell
      (if (Variables|Default|GetIsDestroyingCell)
        (Default|RemovePaintedCell (Variables|Default|GetGameState) (Variables|Default|GetGridCursorPosition))))))

(fn UpdateGridCursorPosition
  (bind _buildgridcursor (Variables|Default|GetBuildGridCursor))
  (bind _gridcellsize (Variables|Default|GetGridCellSize))
  (bind _gridcursorposition (Variables|Default|GetGridCursorPosition))
  (bind _returnvalue (* _gridcellsize _gridcursorposition))
  (Utilities|IsValid _buildgridcursor
    (:Is%20Valid
      (Transformation|SetActorLocation _buildgridcursor _returnvalue false false)
      (Transformation|SetActorLocation (Variables|Default|GetBuildGrid) (Math|Vector|MakeVector 0.0 0.0 (.Z (Math|Vector|BreakVector _returnvalue))) false false))))

(fn DivideFloor
  (params (A :type Vector) (B :type Vector))
  (bind (_x _y _z) (Math|Vector|BreakVector A))
  (bind (_x_2 _y_2 _z_2) (Math|Vector|BreakVector B))
  (return (Math|Vector|MakeVector (Math|Conversions|ToFloat(Integer) (Math|Float|Floor (/ _x _x_2))) (Math|Conversions|ToFloat(Integer) (Math|Float|Floor (/ _y _y_2))) 0.0)))