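; Game state for the level builder game, switching between Build and Simulate modes and forwarding cell painting to the level's Dungeon actor.
; On BeginPlay it finds the first Dungeon, copies its grid cell size to the player pawn, then enters Build.
; ChangeToState fires the matching state-change event only when the state differs.
; Adding or removing painted cells triggers an automatic dungeon rebuild.
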(event EventBeginPlay
  (Utilities|FlowControl|Sequence
    (:then_0
      (bind _outactors (Actor|GetAllActorsOfClass "/Script/DungeonArchitectRuntime.Dungeon"))
      (bind _array_element (Utilities|Array|ForEachLoopwithBreak _outactors :!label _label)
        (:LoopBody
          (Variables|Default|SetDungeon _array_element)
          (goto _label Break))
        (:Completed
          (Utilities|IsValid (Variables|Default|GetDungeon)
            (:Is%20Valid
              (bind _asbp_dalb_pawn (Utilities|Casting|CastToBP_DALB_Pawn (Game|Player|GetPlayerPawn 0)))
              (Variables|/Game/DA_StarterPack/LevelBuilderGame/Blueprints/Game/BP_DALB_Pawn.BP_DALB_Pawn_C|SetGridCellSize _asbp_dalb_pawn (.GridCellSize (Utilities|Struct|BreakDungeonConfig (Variables|/Script/DungeonArchitectRuntime.Dungeon|Getconfig (Variables|Default|GetDungeon))))))))))
    (:then_1
      (CallFunction|ChangetoState "NewEnumerator1"))))

(event EventTick
  (params (DeltaSeconds :type Float%20%28single-precision%29)))

(fn ConstructionScript)

(fn ChangetoState
  (params (State :type DALB_GameStateTypes%20Enum))
  (if (Utilities|Enum|NotEqual(Enum) State (Variables|Default|GetCurrentStateType))
    (bind _output_get (Variables|Default|SetCurrentStateType State))
    (switch Utilities|FlowControl|Switch|SwitchonDALB_GameStateTypes _output_get
      (:NewEnumerator0
        (Default|CallOnStateChangeSimulate))
      (:NewEnumerator1
        (Default|CallOnStateChangeBuild)))))

(fn AddPaintedCell
  (params (Location :type Vector))
  (Class|Dungeon|AddPaintCell (Variables|Default|GetDungeon) Location true))

(fn RemovePaintedCell
  (params (Location :type Vector))
  (Class|Dungeon|RemovePaintCell (Variables|Default|GetDungeon) Location true))