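; Utility Blueprint for the DA query examples that draws a spline path between two dungeon cells from the query's cell path.
; The main builder uses cell centers at both endpoints and each intermediate cell's opening to the next, so the path follows doors and stairs.
; A "SimpleAndUgly" variant uses only cell centers.
; Both append local-space points, update the spline once afterward, then build the actor's spline mesh.
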(fn UpdateSplinePathBetweenCells
  (params (Query :type Grid%20Dungeon%20Query%20Object%20Reference) (CellA :type Integer) (CellB :type Integer) (SplineActor :type BP%20Debug%20Line%20Renderer%20Object%20Reference))
  (bind _outresult (Class|GridDungeonQuery|GetPathBetweenCells Query CellA CellB))
  (for (_array_element _array_index) _outresult
    (if (or (== _array_index 0) (== _array_index (- (Utilities|Array|Length _outresult) 1)))
      ;[1 1 1] Use the cell center if it is the first of the last point
      (Spline|AddSplinePoint (Variables|/Game/DA_Query_Examples/Common/Blueprints/Visuals/BP_DebugLineRenderer.BP_DebugLineRenderer_C|GetSpline SplineActor) (.OutCenter (Class|GridDungeonQuery|GetCellDimension Query _array_element)) "Local" false)
      (else
        ;[1 1 1] Insert a point between the two intersection cells, this way it passes through doors/stairs if needed
        (Spline|AddSplinePoint (Variables|/Game/DA_Query_Examples/Common/Blueprints/Visuals/BP_DebugLineRenderer.BP_DebugLineRenderer_C|GetSpline SplineActor) (Class|GridDungeonQuery|GetOpeningPointBetweenAdjacentCells Query _array_element (Utilities|Array|Get(acopy) _outresult (+ _array_index 1))) "Local" false))))
  ;[1 1 1] Rebuild the spline when done
  (Spline|UpdateSpline (Variables|/Game/DA_Query_Examples/Common/Blueprints/Visuals/BP_DebugLineRenderer.BP_DebugLineRenderer_C|GetSpline SplineActor))
  (Default|BuildSplineMesh SplineActor))

(fn UpdateSplinePathBetweenCellsSimpleandUgly
  (params (Query :type Grid%20Dungeon%20Query%20Object%20Reference) (CellA :type Integer) (CellB :type Integer) (SplineActor :type BP%20Debug%20Line%20Renderer%20Object%20Reference))
  (bind _spline (Variables|/Game/DA_Query_Examples/Common/Blueprints/Visuals/BP_DebugLineRenderer.BP_DebugLineRenderer_C|GetSpline SplineActor))
  (for _array_element (.OutResult (Class|GridDungeonQuery|GetPathBetweenCells Query CellA CellB))
    (Spline|AddSplinePoint _spline (.OutCenter (Class|GridDungeonQuery|GetCellDimension Query _array_element)) "Local" false))
  (Spline|UpdateSpline _spline)
  (Default|BuildSplineMesh SplineActor))