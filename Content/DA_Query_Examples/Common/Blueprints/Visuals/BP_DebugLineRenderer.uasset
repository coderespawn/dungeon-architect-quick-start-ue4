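; BP_DebugLineRenderer is a debug visual actor that draws a line through a stored array of local-space points using spline meshes.
; BuildSplineMesh, also run by the construction script, rebuilds the Spline from SplinePoints and adds one SplineMeshComponent per segment, matched to point locations and tangents.
; AddSplinePoint appends to the array, and ClearSplineMesh empties it and destroys the mesh components.
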(event EventBeginPlay)

(event Collision|EventActorBeginOverlap
  (params (OtherActor :type Actor%20Object%20Reference)))

(event EventTick
  (params (DeltaSeconds :type Float%20%28single-precision%29)))

(fn ConstructionScript
  (CallFunction|BuildSplineMesh))

(fn BuildSplineMesh
  (bind _spline (Variables|Default|GetSpline))
  (bind _spline_2 (Variables|Default|GetSpline))
  ;[1 1 1] Add the spline points to the spline component
  (Spline|ClearSplinePoints (Variables|Default|GetSpline) true)
  (CallFunction|DestroySplineMeshComponents)
  (for _array_element (Variables|Default|GetSplinePoints)
    (Spline|AddSplinePoint _spline _array_element "Local" false))
  (Spline|UpdateSpline _spline)
  ;[1 1 1] Build the spline mesh components for each point
  (for _index (range 0 (- (Spline|GetNumberOfSplinePoints _spline_2) 2))
    (bind _returnvalue (AddComponent|AddSplineMeshComponent true))
    (Transformation|AttachComponentToComponent _returnvalue (Variables|Default|GetDefaultSceneRoot) "None" "KeepRelative" "KeepRelative" "KeepRelative" false)
    (SplineMesh|SetStartandEnd _returnvalue (.Location (Spline|GetLocationandTangentatSplinePoint _spline_2 _index "Local")) (.Tangent (Spline|GetLocationandTangentatSplinePoint _spline_2 _index "Local")) (.Location (Spline|GetLocationandTangentatSplinePoint _spline_2 (+ _index 1) "Local")) (.Tangent (Spline|GetLocationandTangentatSplinePoint _spline_2 (+ _index 1) "Local")) true :!class /Script/Engine.SplineMeshComponent)))

(fn ClearSplineMesh
  (Utilities|Array|Clear (Variables|Default|GetSplinePoints))
  (Spline|ClearSplinePoints (Variables|Default|GetSpline) false)
  (CallFunction|DestroySplineMeshComponents))

(fn AddSplinePoint
  (params (Position :type Vector))
  (Utilities|Array|Add (Variables|Default|GetSplinePoints) Position))

(fn DestroySplineMeshComponents
  (bind _returnvalue (Actor|GetComponentbyClass "/Script/Engine.SplineMeshComponent"))
  (while (Utilities|IsValid _returnvalue)
    (Components|DestroyComponent _returnvalue)
    (Spline|ClearSplinePoints (Variables|Default|GetSpline) true)))