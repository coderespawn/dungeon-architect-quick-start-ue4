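; Example grid dungeon listener that draws a spline path between the two furthest rooms after each dungeon build.
; It gets both rooms and the connecting cell path from the GridDungeonQuery, then feeds points to a LineRenderer spline actor.
; Only the end cells use their centers; openings between adjacent cells supply the other points, routing the line through doors and stairs.
; The spline and its mesh clear on rebuild or dungeon destruction.
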(event EventOnPostDungeonBuild
  (params (Dungeon :type Dungeon%20Object%20Reference))
  (bind _asgrid_dungeon_query (Utilities|Casting|CastToGridDungeonQuery (Class|Dungeon|GetQuery Dungeon)))
  (CallFunction|ClearSpline)
  (CallFunction|UpdateSplinePath _asgrid_dungeon_query (.OutRoomA (Class|GridDungeonQuery|GetFurthestRooms _asgrid_dungeon_query)) (.OutRoomB (Class|GridDungeonQuery|GetFurthestRooms _asgrid_dungeon_query)) (Variables|Default|GetLineRenderer)))

(event EventOnDungeonDestroyed
  (params (Dungeon :type Dungeon%20Object%20Reference))
  (CallFunction|ClearSpline))

(fn UpdateSplinePath
  (params (Query :type Grid%20Dungeon%20Query%20Object%20Reference) (CellA :type Integer) (CellB :type Integer) (SplineActor :type BP%20Debug%20Line%20Renderer%20Object%20Reference))
  (bind _outresult (Class|GridDungeonQuery|GetPathBetweenCells Query CellA CellB))
  (Default|ClearSplineMesh (Variables|Default|GetLineRenderer))
  (for (_array_element _array_index) _outresult
    (if (or (== _array_index 0) (== _array_index (- (Utilities|Array|Length _outresult) 1)))
      ;[1 1 1] Use the cell center if it is the first of the last point
      (Default|AddSplinePoint SplineActor (.OutCenter (Class|GridDungeonQuery|GetCellDimension Query _array_element)))
      (if (== _array_index 0)
        ;[1 1 1] Insert a point between the two intersection cells, this way it passes through doors/stairs if needed
        (Default|AddSplinePoint SplineActor (Class|GridDungeonQuery|GetOpeningPointBetweenAdjacentCells Query _array_element (Utilities|Array|Get(acopy) _outresult (+ _array_index 1))) :!label _label))
      (else
        (goto _label))))
  ;[1 1 1] Rebuild the spline when done
  (Default|BuildSplineMesh SplineActor))

(fn ClearSpline
  (bind _linerenderer (Variables|Default|GetLineRenderer))
  (Spline|ClearSplinePoints (Variables|/Game/DA_Query_Examples/Common/Blueprints/Visuals/BP_DebugLineRenderer.BP_DebugLineRenderer_C|GetSpline _linerenderer) true)
  (Default|ClearSplineMesh _linerenderer))