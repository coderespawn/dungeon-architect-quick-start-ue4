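; Game mode for the GridFlow demo that builds a randomized dungeon at runtime before the match starts.
; On BeginPlay it sets a random seed on the level's Dungeon config and builds it, holding ReadyToStartMatch until completion.
; It then moves and restarts the player at a PlayerStart and rebuilds the controller's minimap.
; Restarted pawns gain an inventory component if missing, and finishing the demo restarts the game.
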(event Custom|OnDungeonBuildComplete
  (params (Dungeon :type Dungeon%20Object%20Reference))
  (Utilities|FlowControl|Sequence
    (:then_0
      ;[1 1 1] Teleport the player to PlayerStart
      (bind _outactors (Actor|GetAllActorsOfClass "/Script/Engine.PlayerStart"))
      (Transformation|Teleport (Game|Player|GetPlayerPawn 0) (.Location (Math|Transform|BreakTransform (Transformation|GetActorTransform (Utilities|Array|Get(acopy) _outactors)))) (.Rotation (Math|Transform|BreakTransform (Transformation|GetActorTransform (Utilities|Array|Get(acopy) _outactors))))))
    (:then_1
      ;[1 1 1] Set a flag so the match can start (See ReadyToStartMatch function)
      (Variables|Default|SetIsDungeonBuilt true)
      (Class|GameModeBase|RestartPlayeratPlayerStart (Game|GetPlayerController 0) (Utilities|Array|Get(acopy) _outactors)))
    (:then_2
      ;[1 1 1] Rebuild the minimap
      (bind _asbp_grid_flow_demo_player_controller (Utilities|Casting|CastToBP_GridFlowDemo_PlayerController (Game|GetPlayerController 0)))
      (Default|RebuildMinimap _asbp_grid_flow_demo_player_controller (Variables|/Script/DungeonArchitectRuntime.Dungeon|GetDungeonModel Dungeon) (Variables|/Script/DungeonArchitectRuntime.Dungeon|GetConfig Dungeon)))))

(event EventBeginPlay
  ;[1 1 1] Randomize and build the dungeon
  (bind _outactors (Actor|GetAllActorsOfClass "/Script/DungeonArchitectRuntime.Dungeon"))
  (bind _output_get (Variables|Default|SetDungeon (Utilities|Array|Get(acopy) _outactors)))
  (EventDispatchers|BindEventtoOnDungeonBuildComplete _output_get (delegate Custom|OnDungeonBuildComplete))
  (bind _asgrid_flow_config (Utilities|Casting|CastToGridFlowConfig (Variables|/Script/DungeonArchitectRuntime.Dungeon|GetConfig _output_get)))
  (Variables|/Script/DungeonArchitectRuntime.DungeonConfig|SetSeed _asgrid_flow_config (Math|Random|RandomInteger 1000000))
  (Class|Dungeon|BuildDungeon _output_get))

(event EventOnRestartPlayer
  (params (NewPlayer :type Controller%20Object%20Reference))
  (bind _returnvalue (Pawn|GetControlledPawn NewPlayer))
  (Utilities|FlowControl|Sequence
    (:then_0
      ;[1 1 1] Add an inventory component to the controlled pawn, if it doesn't already exist
      (Utilities|IsValid (Actor|GetComponentbyClass _returnvalue "/DungeonArchitect/Builders/GridFlowContent/Art/Blueprints/Inventory/GF_InventoryComponent.GF_InventoryComponent_C")
        (:Is%20Not%20Valid
          (AddComponent|AddGFInventoryComponent _returnvalue))))))

(event EventOnGridFlowGameDemoFinish
  (Class|GameMode|RestartGame))

(fn ConstructionScript)

(fn ReadytoStartMatch
  (return (Variables|Default|GetIsDungeonBuilt)))