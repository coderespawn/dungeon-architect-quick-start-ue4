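; Player controller for the Dungeon Architect GridFlow demo game, managing the HUD, minimap and a switch to spectating.
; On BeginPlay it creates the HUD and makes a material instance from a template using the first GridFlowMiniMap actor found.
; RebuildMinimap builds the layout from a given dungeon model and config, then shares that material with the HUD and updates it.
; StartSpectating replaces the controlled pawn with a SpectatorPawn at the same transform.
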(event EventBeginPlay
  (bind _returnvalue (UserInterface|CreateWidget "/Game/DA_GridFlow_Game/UI/UI_GridFowDemo_HUD.UI_GridFowDemo_HUD_C" self))
  (bind _output_get (Variables|Default|SetUI _returnvalue))
  (UserInterface|Viewport|AddtoViewport _output_get 0)
  (bind _outactors (Actor|GetAllActorsOfClass "/Script/DungeonArchitectRuntime.GridFlowMiniMap"))
  (bind _output_get_2 (Variables|Default|SetMiniMap (Utilities|Array|Get(acopy) _outactors)))
  (bind _returnvalue_2 (Class|DungeonMiniMap|CreateMaterialInstancefromTemplate _output_get_2 "/DungeonArchitect/Materials/MiniMap/Material/M_MMGridFlow_Template_Inst.M_MMGridFlow_Template_Inst"))
  (Variables|Default|SetMiniMapMaterial _returnvalue_2))

(fn ConstructionScript)

(fn RebuildMinimap
  (params (DungeonModel :type Dungeon%20Model%20Object%20Reference) (DungeonConfig :type Dungeon%20Config%20Object%20Reference))
  (bind _minimap (Variables|Default|GetMiniMap))
  (Class|DungeonMiniMap|BuildLayout _minimap DungeonModel DungeonConfig)
  (bind _output_get (Variables|/Game/DA_GridFlow_Game/UI/UI_GridFowDemo_HUD.UI_GridFowDemo_HUD_C|SetMiniMapMaterial (Variables|Default|GetUI) (Variables|Default|GetMiniMapMaterial)))
  (Class|DungeonMiniMap|UpdateMaterial _minimap _output_get))

(fn StartSpectating
  (bind _returnvalue (Pawn|GetControlledPawn))
  (Development|PrintString "Start spectating")
  (LocalVariables|SetSpawnPoint (Transformation|GetActorTransform _returnvalue))
  (Actor|DestroyActor _returnvalue)
  (Pawn|UnPossess)
  (bind _returnvalue_2 (Game|SpawnActorfromClass "/Script/Engine.SpectatorPawn" (LocalVariables|GetSpawnPoint) "AdjustIfPossibleButAlwaysSpawn" 0 0))
  (Pawn|Possess _returnvalue_2))