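; BP_StraightLineBuilder is a Dungeon Architect custom builder that generates a straight-line layout of connected rooms.
; On GenerateCustomLayout it clears its state so rebuilds start fresh, then registers a fixed count of rooms along X, spaced by InterRoomDistance with slight random jitter.
; It stores the room IDs and connects each consecutive pair into a linear chain.
; The grid config's cell count is unused.
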(event EventGenerateCustomLayout
  (params (GridConfig :type Grid%20Dungeon%20Config%20Object%20Reference))
  (bind _roomids (Variables|Default|GetRoomIDs))
  (Utilities|FlowControl|Sequence
    (:then_0
      ;[1 1 1] Reset the BP state so the values do not carry over on a next rebuild (Important)
      (Variables|Default|SetCurrentX 0)
      (Utilities|Array|Clear (Variables|Default|GetRoomIDs)))
    (:then_1
      ;[1 1 1] Create the rooms
      (for _index (range 1 20)
        (bind _roomid (Class|GridCustomDungeonBuilder|RegisterRoomat (.OutX (Class|GridCustomDungeonBuilder|GetRandomOffset (Variables|Default|GetCurrentX) 0 1.0)) (.OutY (Class|GridCustomDungeonBuilder|GetRandomOffset (Variables|Default|GetCurrentX) 0 1.0))))
        (Utilities|Array|Add (Variables|Default|GetRoomIDs) _roomid)
        (Variables|Default|SetCurrentX (+ (Variables|Default|GetCurrentX) (Variables|Default|GetInterRoomDistance)))))
    (:then_2
      ;[1 1 1] Connect the rooms
      (for _index_2 (range 0 (- (Utilities|Array|Length (Variables|Default|GetRoomIDs)) 2))
        (Class|GridCustomDungeonBuilder|ConnectRooms (Utilities|Array|Get(acopy) _roomids _index_2) (Utilities|Array|Get(acopy) _roomids (+ _index_2 1)))))))