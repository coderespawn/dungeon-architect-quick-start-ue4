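; Dungeon transform rule that gives placed nodes a random rotation offset, with no change to location or scale.
; GetNodeOffset derives roll, pitch and yaw from random unit vectors scaled by random amounts within plus or minus MaxRotation.
; It draws from the supplied RandomStream, so results follow the seed, and ignores the model, config, cell and grid inputs.
; GetNodeOffsetx is an empty leftover, alongside an unused unseeded transform.
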(fn GetNodeOffsetx
  (return))

(fn GetNodeOffset
  (params (Model :type Grid%20Dungeon%20Model%20Object%20Reference) (Config :type Grid%20Dungeon%20Config%20Object%20Reference) (Cell :type Cell%20Structure%20%28by%20ref%29) (RandomStream :type Random%20Stream%20Structure%20%28by%20ref%29) (GridX :type Integer) (GridY :type Integer))
  (bind _returnvalue (Math|Random|RandomUnitVectorfromStream RandomStream))
  (bind _maxrotation (Variables|Default|GetMaxRotation))
  (bind _returnvalue_2 (* _maxrotation -1.0))
  (bind _returnvalue_3 (Math|Random|RandomFloatinRangefromStream _returnvalue_2 _maxrotation RandomStream))
  (bind _returnvalue_4 (* _returnvalue _returnvalue_3))
  (bind (_x _y _z) (Math|Vector|BreakVector _returnvalue_4))
  (return (Math|Transform|MakeTransform "0, 0, 0" (Math|Rotator|MakeRotator _x _y _z))))