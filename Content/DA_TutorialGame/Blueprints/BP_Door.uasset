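; Double door actor that swings both leaves open when a Pawn enters its trigger and closes them when one leaves.
; Overlap events play or reverse a timeline, which drives UpdateDoorAnim to yaw the two doors in opposite directions up to MaxRotationAngle.
; A cross product picks the swing direction from the side the Pawn is on, and that direction holds until the reverse playback finishes.
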(event OnComponentBeginOverlap(Collide1)
  (params (OtherActor :type Actor%20Object%20Reference) (OtherComp :type Primitive%20Component%20Object%20Reference) (OtherBodyIndex :type Integer) (bFromSweep :type Boolean) (SweepResult :type Hit%20Result%20Structure%20%28by%20ref%29))
  (bind _aspawn (Utilities|Casting|CastToPawn OtherActor))
  (Variables|Default|SetNearbyActor _aspawn)
  (bind (_direction _dooropenratio) (Timeline|Timeline_0 Play)
    (:Update
      (CallFunction|UpdateDoorAnim _dooropenratio))
    (:Finished
      (if (Utilities|Enum|Equal(Enum) _direction "Backward")
        (Variables|Default|SetDirection 0)))))

(event OnComponentEndOverlap(Collide1)
  (params (OtherActor :type Actor%20Object%20Reference) (OtherComp :type Primitive%20Component%20Object%20Reference) (OtherBodyIndex :type Integer))
  (Utilities|Casting|CastToPawn OtherActor)
  (bind (_direction _dooropenratio) (Timeline|Timeline_0 Reverse)
    (:Update
      (CallFunction|UpdateDoorAnim _dooropenratio))
    (:Finished
      (if (Utilities|Enum|Equal(Enum) _direction "Backward")
        (Variables|Default|SetDirection 0)))))

(event EventBeginPlay)

(event EventActorBeginOverlap
  (params (OtherActor :type Actor%20Object%20Reference)))

(event EventTick
  (params (DeltaSeconds :type Float%20%28single-precision%29)))

(fn ConstructionScript)

(fn UpdateDoorAnim
  (params (Ratio :type Float%20%28single-precision%29))
  (CallFunction|CalculateDirection)
  (LocalVariables|SetCurrentAngle (* Ratio (Variables|Default|GetMaxRotationAngle)))
  (Transformation|SetRelativeRotation (Variables|Default|GetDoor1) (Math|Rotator|MakeRotator 0.0 0.0 (* (Variables|Default|GetDirection) (LocalVariables|GetCurrentAngle))) false false)
  (Transformation|SetRelativeRotation (Variables|Default|GetDoor2) (Math|Rotator|MakeRotator 0.0 0.0 (* (* (Variables|Default|GetDirection) (LocalVariables|GetCurrentAngle)) -1.0)) false false))

(fn CalculateDirection
  (if (== (Variables|Default|GetDirection) 0)
    (if (> (.Z (Math|Vector|BreakVector (Math|Vector|CrossProduct (Math|Vector|Normalize (- (Transformation|GetActorLocation (Variables|Default|GetNearbyActor)) (Transformation|GetActorLocation))) (Math|Vector|RotateVector (Math|Vector|MakeVector 0.0 -1.0 0.0) (Transformation|GetActorRotation))))) 0.0)
      (Variables|Default|SetDirection 1)
      (else
        (Variables|Default|SetDirection -1)))))