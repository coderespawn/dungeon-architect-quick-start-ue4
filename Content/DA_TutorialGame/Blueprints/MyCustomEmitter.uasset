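; A Dungeon Architect marker emitter for the tutorial game that adds a custom marker at the center of each room in a grid dungeon.
; It casts the config and model to their grid types, then loops over the cells and keeps only Room cells.
; Each room's bounds are converted to world coordinates using the grid cell size, and a MyRoomCenter marker is emitted at location plus half size.
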(event EventEmitMarkers
  (params (Builder :type Dungeon%20Builder%20Object%20Reference) (Model :type Dungeon%20Model%20Object%20Reference) (Config :type Dungeon%20Config%20Object%20Reference))
  (bind _asgrid_dungeon_config (Utilities|Casting|CastToGridDungeonConfig Config))
  (Variables|Default|SetGridSize (Variables|/Script/DungeonArchitectRuntime.GridDungeonConfig|GetGridCellSize _asgrid_dungeon_config))
  (bind _asgrid_dungeon_model (Utilities|Casting|CastToGridDungeonModel Model))
  (for _array_element (Variables|/Script/DungeonArchitectRuntime.GridDungeonModel|GetCells _asgrid_dungeon_model)
    (if (Utilities|Enum|Equal(Enum) (.CellType (Utilities|Struct|BreakCell _array_element)) "Room")
      (Class|DungeonBuilder|EmitMarker Builder "MyRoomCenter" (Math|Transform|MakeTransform (+ (.Location (Class|GridDungeonModelHelper|ToWorldCoords (.Bounds (Utilities|Struct|BreakCell _array_element)) (Variables|Default|GetGridSize))) (/ (.Size (Class|GridDungeonModelHelper|ToWorldCoords (.Bounds (Utilities|Struct|BreakCell _array_element)) (Variables|Default|GetGridSize))) 2.0)))))))