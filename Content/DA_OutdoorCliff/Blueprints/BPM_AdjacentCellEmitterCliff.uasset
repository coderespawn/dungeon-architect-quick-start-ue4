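; Dungeon Architect marker emitter for grid dungeons that marks the empty cells surrounding the layout, out to DistanceToCover rings.
; EmitMarkers clears AdjacentCells, then runs AddBorderEmitters per ring, expanding each cell's bounds and keeping border points of Unknown type.
; Each new point gets a generic EmptySpace marker plus a distance-indexed one at its grid center.
; AdjacentCells deduplicates by XY position, so inner rings take priority.
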(event EventEmitMarkers
  (params (Builder :type Dungeon%20Builder%20Object%20Reference) (Model :type Dungeon%20Model%20Object%20Reference) (Config :type Dungeon%20Config%20Object%20Reference))
  (Utilities|Array|Clear (Variables|Default|GetAdjacentCells))
  (for _index (range 1 (Variables|Default|GetDistanceToCover))
    (CallFunction|AddBorderEmitters _index Builder Model Config)))

(fn AddBorderEmitters
  (params (Level :type Integer) (Builder :type Dungeon%20Builder%20Object%20Reference) (Model :type Dungeon%20Model%20Object%20Reference) (Config :type Dungeon%20Config%20Object%20Reference))
  (bind _asgrid_dungeon_config (Utilities|Casting|CastToGridDungeonConfig Config))
  (bind _asgrid_dungeon_model (Utilities|Casting|CastToGridDungeonModel Model))
  (bind _asgrid_dungeon_builder (Utilities|Casting|CastToGridDungeonBuilder Builder))
  (LocalVariables|SetDistance Level)
  (for _array_element (Variables|/Script/DungeonArchitectRuntime.GridDungeonModel|GetCells _asgrid_dungeon_model)
    (for _array_element_2 (Class|DungeonModelHelper|GetRectBorderPoints (Class|DungeonModelHelper|ExpandBounds (.Bounds (Utilities|Struct|BreakCell _array_element)) (LocalVariables|GetDistance)))
      (if (not (Utilities|Enum|NotEqual(Enum) (.CellType (Utilities|Struct|BreakGridCellInfo (Class|GridDungeonModel|GetGridCellLookup _asgrid_dungeon_model (.X (Utilities|Struct|BreakIntVector _array_element_2)) (.Y (Utilities|Struct|BreakIntVector _array_element_2))))) "Unknown"))
        (if (not (Utilities|Array|ContainsItem (Variables|Default|GetAdjacentCells) (Math|Vector|MakeVector (.X (Math|Vector|BreakVector (* (+ (Class|DungeonModelHelper|MakeVector _array_element_2 1.0) "0.500000,0.500000, 0") (Variables|/Script/DungeonArchitectRuntime.GridDungeonConfig|GetGridCellSize _asgrid_dungeon_config)))) (.Y (Math|Vector|BreakVector (* (+ (Class|DungeonModelHelper|MakeVector _array_element_2 1.0) "0.500000,0.500000, 0") (Variables|/Script/DungeonArchitectRuntime.GridDungeonConfig|GetGridCellSize _asgrid_dungeon_config)))) 0.0)))
          (Utilities|Array|Add (Variables|Default|GetAdjacentCells) (Math|Vector|MakeVector (.X (Math|Vector|BreakVector (* (+ (Class|DungeonModelHelper|MakeVector _array_element_2 1.0) "0.500000,0.500000, 0") (Variables|/Script/DungeonArchitectRuntime.GridDungeonConfig|GetGridCellSize _asgrid_dungeon_config)))) (.Y (Math|Vector|BreakVector (* (+ (Class|DungeonModelHelper|MakeVector _array_element_2 1.0) "0.500000,0.500000, 0") (Variables|/Script/DungeonArchitectRuntime.GridDungeonConfig|GetGridCellSize _asgrid_dungeon_config)))) 0.0))
          (Class|DungeonBuilder|EmitMarker _asgrid_dungeon_builder "EmptySpace" (Math|Transform|MakeTransform (* (+ (Class|DungeonModelHelper|MakeVector _array_element_2 1.0) "0.500000,0.500000, 0") (Variables|/Script/DungeonArchitectRuntime.GridDungeonConfig|GetGridCellSize _asgrid_dungeon_config))))
          (Class|DungeonBuilder|EmitMarker _asgrid_dungeon_builder (Utilities|String|ToString(Text) (Utilities|Text|FormatText "EmptySpace{Index}" (Utilities|Text|ToText(Integer) (LocalVariables|GetDistance)))) (Math|Transform|MakeTransform (* (+ (Class|DungeonModelHelper|MakeVector _array_element_2 1.0) "0.500000,0.500000, 0") (Variables|/Script/DungeonArchitectRuntime.GridDungeonConfig|GetGridCellSize _asgrid_dungeon_config)))))))))